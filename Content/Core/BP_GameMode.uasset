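; BP_GameMode is the game mode that tracks the player's points and decides which ending plays.
; AddPoint increments the Points counter, while GameEnd calls CallBPOnGameEnd and then checks whether Points equals exactly three.
; A match shows the good-ending widget with the win sound; otherwise it shows the bad-ending widget with the lose sound, and either widget then runs GoBackToMenu.
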(event Custom|AddPoint
  (Variables|Default|SetPoints (+ (Variables|Default|GetPoints) 1)))

(event Custom|GameEnd
  (Default|CallBPonGameEnd)
  (if (== (Variables|Default|GetPoints) 3)
    (bind _returnvalue (UserInterface|CreateWidget "/Game/UI/Widgets/W_GoodEnding.W_GoodEnding_C"))
    (UserInterface|Viewport|AddtoViewport _returnvalue 0)
    (Audio|PlaySound2D "/Game/Sounds/Cues/CUE_Win.CUE_Win" 1.0 1.0 0.0 0 0)
    (Default|GoBacktoMenu _returnvalue)
    (else
      (bind _returnvalue_2 (UserInterface|CreateWidget "/Game/UI/Widgets/W_BadEnding.W_BadEnding_C"))
      (UserInterface|Viewport|AddtoViewport _returnvalue_2 0)
      (Audio|PlaySound2D "/Game/Sounds/Cues/CUE_Lose.CUE_Lose" 1.0 1.0 0.0 0 0)
      (Default|GoBacktoMenu _returnvalue_2))))

(event EventBeginPlay)

(event EventTick
  (params (DeltaSeconds :type Float%20%28single-precision%29)))

(fn ConstructionScript)