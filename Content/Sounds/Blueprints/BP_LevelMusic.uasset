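; BP_LevelMusic is an actor that controls a level's music and ambiance audio.
; On BeginPlay it binds to event dispatchers on BP_GameMode and the BP_Descartes player pawn.
; Game end stops both music and ambiance, while the pawn's events stop only the music or play it again from the start.
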(event Custom|BP_StopMusic
  (Audio|Components|Audio|Stop (Variables|Default|GetMusicAudioComponent))
  (Audio|Components|Audio|Stop (Variables|Default|GetAmbianceAudioComponent)))

(event Custom|BP_StartMusic
  (Audio|Components|Audio|Play (Variables|Default|GetMusicAudioComponent) 0.0))

(event Custom|BP_OnlyStopLevelMusic
  (Audio|Components|Audio|Stop (Variables|Default|GetMusicAudioComponent)))

(event EventBeginPlay
  (bind _asbp_game_mode (Utilities|Casting|CastToBP_GameMode (Game|GetGameMode)))
  (EventDispatchers|BindEventtoBPonGameEnd _asbp_game_mode (delegate Custom|BP_StopMusic))
  (bind _asbp_descartes (Utilities|Casting|CastToBP_Descartes (Game|Player|GetPlayerPawn 0)))
  (EventDispatchers|BindEventtoBPEndMusic _asbp_descartes (delegate Custom|BP_OnlyStopLevelMusic))
  (EventDispatchers|BindEventtoBPStartMusicAgain _asbp_descartes (delegate Custom|BP_StartMusic)))

(event Collision|EventActorBeginOverlap
  (params (OtherActor :type Actor%20Object%20Reference)))

(event EventTick
  (params (DeltaSeconds :type Float%20%28single-precision%29)))

(fn ConstructionScript)